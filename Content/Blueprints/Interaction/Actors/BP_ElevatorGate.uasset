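; Elevator gate actor that slides its Item component vertically between open and closed using a Timeline-driven lerp on relative Z.
; BeginPlay triggers the open/close toggle and plays DoorOpen_TL, which updates IsDoorOpen from its direction after a short delay and enables interaction.
; The toggle plays or reverses that timeline according to IsDoorOpen.
; Interacts is a debug path with its own timeline, and a player-facing dot product is left unconnected.
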(event `/Game/Blueprints/Interfaces/BPI_Interacts.Interacts`
  (params (interactionActor :type "Character Object Reference"))
  (bind _item (`self.Item`))
  (bind (_returnvalue_x _returnvalue_y) (`KismetMathLibrary.BreakVector` (`SceneComponent.K2_GetComponentLocation` _item)))
  ;[0.05616 1 0.2499] debugging
  (`Timeline|Timeline` :`NewTime` 5.0
    (:`Update`
      (`SceneComponent.K2_SetRelativeLocation` (`self.Item`) (100.0 90.0 50.0) false false)
      (`SceneComponent.K2_SetRelativeLocation` _item (`KismetMathLibrary.MakeVector` _returnvalue_x _returnvalue_y (`KismetMathLibrary.Lerp` -100.0 0.0 (stale `self.ReceiveBeginPlay` _alpha))) false false :!label _label))))

(event `self.ReceiveBeginPlay`
  (`self.Open/CloseDoor`)
  (bind (_direction _alpha) (`Timeline|DoorOpen_TL` :`NewTime` 2.0 :!label _label_2)
    (:`Update`
      (goto _label))
    (:`Finished`
      (`KismetSystemLibrary.Delay` 0.3)
      (switch `ETimelineDirection` _direction
        (:`Forward`
          (set `self.IsDoorOpen?` true))
        (:`Backward`
          (set `self.IsDoorOpen?` false)))
      (set `self.CanInteract?_0` true))))

(event `Open/CloseDoor`
  ;[1 0.4069 0.9939] Check if the door is can be opened?
  (if (`self.CanInteract?_0`)
    (set `self.CanInteract?_0` true)
    (if (not (`self.IsDoorOpen?`))
      (goto _label_2 :!via `PlayFromStart`)
      (else
        (goto _label_2 :!via `ReverseFromEnd`)))))

(fn `UserConstructionScript`
  (`parent.UserConstructionScript`))