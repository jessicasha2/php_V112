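; BP_Item_Master is an item actor, named as the master for items, that the player picks up by interacting with it.
; The construction script fills ItemInformation from the DT_ItemData row matching the ItemNames enum.
; Interacts passes that data to the player's BP_MysteryChar through ItemPickup, then destroys the actor.
; CanInteract always returns false, and PickUpItem only prints a debug string and triggers a briefly delayed destroy.
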(event `DestroyItem`
  (`KismetSystemLibrary.Delay` 0.1)
  (`self.K2_DestroyActor`))

(event `/Game/Blueprints/Interfaces/BPI_Interacts.Interacts`
  (params (interactionActor :type "Character Object Reference"))
  (bind _asbp_mystery_char (cast `/Game/Blueprints/GAME/BP_MysteryChar` (`GameplayStatics.GetPlayerCharacter` 0)))
  (`/Game/Blueprints/GAME/BP_MysteryChar.ItemPickup` _asbp_mystery_char (`self.ItemInformation`))
  (`self.K2_DestroyActor`))

(fn `CanInteract?`
  (returns (`Interactable?` :type Boolean))
  (return false))

(fn `PickUpItem`
  (params (ItemClass :type "Actor Class Reference") (StackAmount :type Integer) (ItemIcon :type "Texture2D Object Reference") (MaxStackAmount :type Integer))
  (returns (Item :type String))
  (`KismetSystemLibrary.PrintString` "item")
  (`self.DestroyItem`)
  (return ""))

(fn `UserConstructionScript`
  (bind _returnvalue (`|GetDataTableRow` "/Game/DataTables/DT_ItemData.DT_ItemData" (`KismetStringLibrary.Conv_StringToName` (`|GetEnumeratorNameAsString` (`self.ItemNames`))))
    (:`then`
      (set `self.ItemInformation` _returnvalue))))