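; An interactable double door that swings both leaves open away from the player and closes them on the next interaction.
; On opening, a dot product of the player-to-door direction and the door's forward vector picks the swing side.
; A timeline lerps mirrored yaw rotations on both leaves and plays in reverse to close.
; A lock flag blocks interaction until shortly after each swing finishes.
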(event `/Game/Blueprints/Interfaces/BPI_Interacts.Interacts`
  (params (interactionActor :type "Character Object Reference"))
  (`self.Open/CloseDoor`))

(event `Open/CloseDoor`
  ;[1 0.4069 0.9939] Check if the door is can be opened?
  (if (`self.CanInteract?_0`)
    (set `self.CanInteract?_0` false)
    (if (not (`self.IsDoorOpen?`))
      (set `self.DotProduct` (`KismetMathLibrary.Dot_VectorVector` (`KismetMathLibrary.Normal` (- (`self.K2_GetActorLocation` self) (`self.K2_GetActorLocation` (`self.Player_Char_REF`)))) (`self.GetActorForwardVector` self)))
      (bind (_direction _alpha) (`Timeline|DoorOpen_TL` :!via `PlayFromStart` :!label _label)
        (:`Update`
          (bind _returnvalue (`KismetMathLibrary.Lerp` 0.0 (* (select `bool` (>= (`self.DotProduct`) 0.0) :`false` 90.0 :`true` -90.0) -1.0) _alpha))
          (`SceneComponent.K2_SetRelativeRotation` (`self.doorL`) (`KismetMathLibrary.MakeRotator` 0.0 0.0 _returnvalue) false false)
          (`SceneComponent.K2_SetRelativeRotation` (`self.door`) (`KismetMathLibrary.MakeRotator` 0.0 0.0 (* _returnvalue -1.0)) false false))
        (:`Finished`
          (`KismetSystemLibrary.Delay` 0.3)
          (switch `ETimelineDirection` _direction
            (:`Forward`
              (set `self.IsDoorOpen?` true))
            (:`Backward`
              (set `self.IsDoorOpen?` false)))
          (set `self.CanInteract?_0` true)))
      (else
        (goto _label :!via `ReverseFromEnd`)))))

(fn `UserConstructionScript`
  (`parent.UserConstructionScript`))