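; BP_LightSwitch is an interactable light switch that turns its assigned lights on and off.
; Its Interacts event loops over the Light array, skips invalid entries and flips each light component's visibility.
; Each light toggles from its own current state, so lights that start in mixed states stay mixed.
; BeginPlay, overlap and Tick are unused, leaving the switch purely event-driven.
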(event `/Game/Blueprints/Interfaces/BPI_Interacts.Interacts`
  (params (interactionActor :type "Character Object Reference"))
  ;[1 1 1] for use on multiple lights
  (for _array_element (`self.Light`)
    (`/Engine/EditorBlueprintResources/StandardMacros.IsValid` _array_element
      (:`Is Valid`
        (bind _lightcomponent (`Light.LightComponent` _array_element))
        (if (`SceneComponent.IsVisible` _lightcomponent)
          (`SceneComponent.SetVisibility` _lightcomponent false false)
          (else
            (`SceneComponent.SetVisibility` _lightcomponent true false)))))))

(fn `UserConstructionScript`
  (`parent.UserConstructionScript`))