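; BP_HideActor_Master is a possessable base hiding spot that lets the player hide in it.
; The UnderObject overlap tracks the player and gates the Interacts event, which hides the player, blends the view to this actor, then possesses it.
; IA_InteractWith repossesses the player pawn, moves the player to ExitLoc and unhides it.
; CanInteract always returns false, and older BP_MysteryChar hide logic remains unconnected.
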(event `self.UnderObject.OnComponentBeginOverlap`
  (params (OverlappedComponent :type "PrimitiveComponent Object Reference") (OtherActor :type "Actor Object Reference") (OtherComp :type "PrimitiveComponent Object Reference") (OtherBodyIndex :type Integer) (bFromSweep :type Boolean) (SweepResult :type "HitResult Structure (by ref)"))
  (if (`self.ActorHasTag` OtherActor "Player")
    (set `self.CanHide?` true)
    (set `self.playerActor` OtherActor)
    (set `self.playerPawn` (`GameplayStatics.GetPlayerPawn` 0))))

(event `self.UnderObject.OnComponentEndOverlap`
  (params (OverlappedComponent :type "PrimitiveComponent Object Reference") (OtherActor :type "Actor Object Reference") (OtherComp :type "PrimitiveComponent Object Reference") (OtherBodyIndex :type Integer))
  (if (`self.ActorHasTag` OtherActor "Player")
    (if (not (`self.isundertable`))
      (set `self.CanHide?` false)
      (set `self.playerActor` null)
      (set `self.playerPawn` null))))

(event `/Game/Blueprints/Interfaces/BPI_Interacts.Interacts`
  (params (interactionActor :type "Character Object Reference"))
  (bind _returnvalue (`GameplayStatics.GetPlayerController` 0))
  ;[1 1 1] changing char position
  (if (`self.isundertable`)
    _
    (elif (`self.CanHide?`)
      (set `self.isundertable` true)
      (`self.SetActorHiddenInGame` (`self.playerActor`) true)
      (`PlayerController.SetViewTargetWithBlend` (`GameplayStatics.GetPlayerController` 0) self 1.0 "VTBlend_Linear" 0.0 false)
      ;[1 1 1] change char to cam and transistion
      (`KismetSystemLibrary.Delay` 1.0)
      (`Controller.UnPossess` _returnvalue)
      (`Controller.Possess` _returnvalue self))))

(event `EnhancedInput|/Game/Blueprints/Inputs/Actions/IA_InteractWith`
  (params (ActionValue :type Boolean) (ElapsedSeconds :type "Float (double-precision)") (TriggeredSeconds :type "Float (double-precision)") (InputAction :type "InputAction Object Reference" :default "/Game/Blueprints/Inputs/Actions/IA_InteractWith.IA_InteractWith"))
  (bind _returnvalue (`GameplayStatics.GetPlayerController` 0))
  (bind _exitloc (`self.ExitLoc`))
  ;[1 1 1] Unpossession
  (:`Started`
    (if (`self.isundertable`)
      (`Controller.UnPossess` _returnvalue)
      (`Controller.Possess` _returnvalue (`self.playerPawn`))
      (`self.K2_SetActorLocationAndRotation` (`self.playerActor`) (`SceneComponent.K2_GetComponentLocation` _exitloc) (`SceneComponent.K2_GetComponentRotation` _exitloc) false false)
      (`self.SetActorHiddenInGame` (`self.playerActor`) false)
      (set `self.isundertable` false))))

(fn `CanInteract?`
  (returns (`Interactable?` :type Boolean))
  (return false))

(fn `UserConstructionScript`)