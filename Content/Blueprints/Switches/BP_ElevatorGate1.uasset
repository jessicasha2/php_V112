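; BP_ElevatorGate1 is a switch-driven gate that opens or closes according to how many switches are active.
; GateActivated and GateDeactivated raise or lower the active count and print debug strings.
; Both then compare it to the required number, playing Gate_TL when met and reversing it otherwise, with the timeline driving relative X location.
; A disconnected delayed BarrierDown_TL chain for vertical movement never runs.
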(event `self.ReceiveTick`
  (params (DeltaSeconds :type "Float (single-precision)"))
  ;[1 1 1] debugging
)

(event `GateActivated`
  (`KismetSystemLibrary.PrintString` "gateActivated")
  (`/Engine/EditorBlueprintResources/StandardMacros.IncrementInt` (`self.NumSwitchActivated`)
    (:`  `
      (if (>= (`self.NumSwitchActivated`) (`self.NumSwitchesNeeded`))
        (bind (_direction _alpha) (`Timeline|Gate_TL` :!label _label)
          (:`Update`
            (`SceneComponent.K2_SetRelativeLocation` (`KismetMathLibrary.MakeVector` _alpha))))
        (else
          (goto _label :!via `Reverse`))))))

(event `GateDeactivated`
  (`KismetSystemLibrary.PrintString` "gateDeactivated")
  (`/Engine/EditorBlueprintResources/StandardMacros.DecrementInt` (`self.NumSwitchActivated`)
    (:`  `
      (if (>= (`self.NumSwitchActivated`) (`self.NumSwitchesNeeded`))
        (goto _label)
        (else
          (goto _label :!via `Reverse`))))))

(fn `UserConstructionScript`)