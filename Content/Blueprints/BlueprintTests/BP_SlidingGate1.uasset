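; Sliding gate Blueprint that opens and closes by moving ElevatorGate1 along its relative Z axis.
; ToggleDoor picks OpenGate or CloseGate from the current direction of the GateMvmt_TL timeline, which they play or reverse.
; The timeline's Alpha feeds the gate's Z location directly.
; On finish, it sets IsOpen true when forward, or IsClosed false when backward.
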(event `self.ReceiveBeginPlay`)

(event `ToggleDoor`
  (switch `ETimelineDirection` (stale `OpenGate` _direction)
    (:`Forward`
      (`self.CloseGate`))
    (:`Backward`
      (`self.OpenGate`))))

(event `OpenGate`
  (bind (_direction _alpha) (`Timeline|GateMvmt_TL` :!label _label)
    (:`Update`
      (`SceneComponent.K2_SetRelativeLocation` (`self.ElevatorGate1`) (`KismetMathLibrary.MakeVector` 0.0 0.0 _alpha) false false))
    (:`Finished`
      (switch `ETimelineDirection` _direction
        (:`Forward`
          (set `self.isOpen?` true))
        (:`Backward`
          (set `self.isClosed?` false))))))

(event `CloseGate`
  (goto _label :!via `Reverse`))

(fn `UserConstructionScript`)