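; Player movement component that handles walking, sprinting and crouching, using sanity as the sprint resource.
; Sprinting needs sanity, movement and ground contact, then a looping timer drains sanity until it runs out or the player slows.
; Stopping while not crouched restores walk speed and, after a retriggerable delay, starts a timer that refills sanity.
; Crouching cancels the sprint timer, changes speed and has the player reference resize its capsule.
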(event `StartSprinting`
  (bind _player_ref (`self.Player_REF`))
  ;[0.8785 0.05796 0.482] Comment
  ;;[0.6249 0.4297 1] Start Sprinting
  (`KismetSystemLibrary.PrintString` "start sprint")
  (if (and (> (`self.CurrentSanity`) (`self.MinSanity`)) (> (`KismetMathLibrary.VSize` (`Actor.GetVelocity` _player_ref)) 10.0) (not (`NavMovementComponent.IsFalling` (`Character.CharacterMovement` _player_ref))))
    (`self.SetMaxWalkSpeed` (`self.SprintSpeed`))
    (`KismetSystemLibrary.K2_SetTimer` null "SprintTimer" 0.1 true)))

(event `SprintTimer`
  ;[0.2299 0.6145 1] How long can you sprint?
  (bind _output_get (set `self.CurrentSanity` (`KismetMathLibrary.FClamp` (- (`self.CurrentSanity`) 1.0) (`self.MinSanity`) (`self.MaxSanity`))))
  (`KismetSystemLibrary.PrintString` (`KismetStringLibrary.Conv_DoubleToString` _output_get) false false)
  (if (<= (`self.CurrentSanity`) (`self.MinSanity`))
    (`self.StopSprinting` :!label _label)
    (elif (not (and (> (`self.CurrentSanity`) (`self.MinSanity`)) (> (`KismetMathLibrary.VSize` (`Actor.GetVelocity` (`self.Player_REF`))) 10.0)))
      (goto _label))))

(event `StopSprinting`
  ;[0.5105 0.4209 1] Comment
  ;;[1 1 1] Stop Sprinting
  (`KismetSystemLibrary.PrintString` "stop sprint")
  (if (not (`self.IsCrouching?`))
    (`KismetSystemLibrary.K2_ClearTimer` null "SprintTimer")
    (`self.SetMaxWalkSpeed` (`self.WalkSpeed`))
    (`KismetSystemLibrary.RetriggerableDelay` 5.0)
    (if (not (`KismetSystemLibrary.K2_IsTimerActive` null "SprintTimer"))
      ;;[1 1 1] check this later
      (`KismetSystemLibrary.K2_SetTimer` null "RegenerateSanity" 0.03 true))))

(event `RegenerateSanity`
  ;[0.926 0.4855 1] Sanity Regenerations, if only this worked in real life
  (bind _output_get (set `self.CurrentSanity` (`KismetMathLibrary.FClamp` (+ (`self.CurrentSanity`) 1.0) (`self.MinSanity`) (`self.MaxSanity`))))
  ;[1 1 1] Debugging
  (`KismetSystemLibrary.PrintString` "RegenerateSanityCurrent Sanity")
  (`KismetSystemLibrary.PrintString` (`KismetStringLibrary.Conv_DoubleToString` _output_get))
  (if (>= (`self.CurrentSanity`) (`self.MaxSanity`))
    (`KismetSystemLibrary.K2_ClearTimer` null "RegenerateSanity")))

(event `StartCrouch`
  ;[1 0.9359 0.09279] Work on crouch logic start Crouch never being called
  (set `self.IsCrouching?` true)
  (`KismetSystemLibrary.K2_ClearTimer` null "SprintTimer")
  (`self.SetMaxWalkSpeed` (`self.CrouchSpeed`))
  (`/Game/Blueprints/GAME/BP_MysteryChar.ShortenCapsuleHeight` (`self.Player_REF`)))

(event `EndCrouch`
  ;[1 0.9359 0.09279] Work on crouch logic start Crouch never being called
  (set `self.IsCrouching?` false)
  (`self.SetMaxWalkSpeed` (`self.WalkSpeed`))
  (`/Game/Blueprints/GAME/BP_MysteryChar.LengthenCapsuleHeight` (`self.Player_REF`)))

(fn `Initialize`
  (params (Player_REF :type "/Game/Blueprints/GAME/BP_MysteryChar Object Reference"))
  (bind _output_get (set `self.Player_REF` Player_REF))
  (set `CharacterMovementComponent.MaxWalkSpeed` (`self.WalkSpeed`) (`Character.CharacterMovement` _output_get)))

(fn `SetMaxWalkSpeed`
  (params (MaxWalkSpeed :type "Float (double-precision)"))
  (set `CharacterMovementComponent.MaxWalkSpeed` MaxWalkSpeed (`Character.CharacterMovement` (`self.Player_REF`))))

(fn `StopSprint`)