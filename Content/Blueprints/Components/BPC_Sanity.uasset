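; BPC_Sanity is a component that holds a sanity value and exposes functions to change it.
; IncreaseSanity adds an amount to CurrentSanity, while DecreaseSanity subtracts CurrentSanity from the damage amount, reversing the expected operand order.
; Both clamp the result between MinSanity and MaxSanity, store it and return it.
; UpdateSanity is an empty stub, and the event graph has no active logic.
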(fn `DecreaseSanity`
  (params (DamageSanity :type "Float (double-precision)"))
  (returns (NewSanity :type "Float (double-precision)"))
  (bind _output_get (set `self.CurrentSanity` (`KismetMathLibrary.FClamp` (- DamageSanity (`self.CurrentSanity`)) (`self.MinSanity`) (`self.MaxSanity`))))
  (return _output_get))

(fn `IncreaseSanity`
  (params (IncreaseSanity :type "Float (double-precision)"))
  (returns (NewSanity :type "Float (double-precision)"))
  (bind _output_get (set `self.CurrentSanity` (`KismetMathLibrary.FClamp` (+ (`self.CurrentSanity`) IncreaseSanity) (`self.MinSanity`) (`self.MaxSanity`))))
  (return _output_get))

(fn `UpdateSanity`)