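; BPC_Dialogue is a dialogue component that supplies conversation lines to the player character.
; Its Conversation event checks that the player is not already speaking, then sends the Dialogue entry at DialoguePosition with a text display delay through TalkingMessage.
; DialoguePosition resets to zero at the last entry, but nothing in this graph advances it.
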(event `Conversation`
  (bind _returnvalue (`GameplayStatics.GetPlayerCharacter` 0))
  (bind _isspeaking_ (message `/Game/Blueprints/Interfaces/BPI_Communicate.CheckIfSpeaking` _returnvalue))
  (if (not _isspeaking_)
    (message `/Game/Blueprints/Interfaces/BPI_Communicate.Talking` _returnvalue (`|GetArrayItem` (`self.Dialogue`) (`self.DialoguePosition`)) (`self.TextDisplayDelay`))
    (if (>= (+ (`self.DialoguePosition`) 1) (`KismetArrayLibrary.Array_Length` (`self.Dialogue`)))
      (set `self.DialoguePosition` 0))))