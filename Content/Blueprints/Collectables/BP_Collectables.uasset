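; BP_Collectables is a collectable pickup that the player collects with the interact input while standing in its trigger box.
; Box overlaps with BP_MysteryChar enable and disable the actor's input, so IA_InteractWith only responds nearby.
; Interacting decrements RemainingCollectables on BP_MysteryGameMode, adds a W_Collectables widget to the viewport and destroys the actor.
; An inventory-style PickUpItemMessage call is left unconnected and never runs.
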(event `self.Box.OnComponentBeginOverlap`
  (params (OverlappedComponent :type "PrimitiveComponent Object Reference") (OtherActor :type "Actor Object Reference") (OtherComp :type "PrimitiveComponent Object Reference") (OtherBodyIndex :type Integer) (bFromSweep :type Boolean) (SweepResult :type "HitResult Structure (by ref)"))
  (cast `/Game/Blueprints/GAME/BP_MysteryChar` OtherActor)
  (`self.EnableInput` (`GameplayStatics.GetPlayerController` 0)))

(event `self.Box.OnComponentEndOverlap`
  (params (OverlappedComponent :type "PrimitiveComponent Object Reference") (OtherActor :type "Actor Object Reference") (OtherComp :type "PrimitiveComponent Object Reference") (OtherBodyIndex :type Integer))
  (cast `/Game/Blueprints/GAME/BP_MysteryChar` OtherActor)
  (`self.DisableInput` (`GameplayStatics.GetPlayerController` 0)))

(event `EnhancedInput|/Game/Blueprints/Inputs/Actions/IA_InteractWith`
  (params (ActionValue :type Boolean) (ElapsedSeconds :type "Float (double-precision)") (TriggeredSeconds :type "Float (double-precision)") (InputAction :type "InputAction Object Reference" :default "/Game/Blueprints/Inputs/Actions/IA_InteractWith.IA_InteractWith"))
  (:`Started`
    (bind _asbp_mystery_game_mode (cast `/Game/Blueprints/GAME/BP_MysteryGameMode` (`GameplayStatics.GetGameMode`)))
    (bind _result (`/Engine/EditorBlueprintResources/StandardMacros.DecrementInt` (`/Game/Blueprints/GAME/BP_MysteryGameMode.RemainingCollectables` _asbp_mystery_game_mode))
      (:`  `
        (set `/Game/Blueprints/GAME/BP_MysteryGameMode.RemainingCollectables` _result _asbp_mystery_game_mode)
        (bind _returnvalue (`|CreateWidget` "/Game/Widgets/UMG/W_Collectables.W_Collectables_C"))
        (`UserWidget.AddToViewport` _returnvalue 0)
        (`self.K2_DestroyActor`)))))

(fn `UserConstructionScript`)